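; Terrain tile for an infinite-terrain game that fills itself with randomized props and AI characters and gates the player with a barrier.
; On BeginPlay it locks, then scatters containers, rocks, boxes, sandbags, canisters and characters.
; The player's overlap with LockingVolume toggles barrier collision and red/green material.
; Player entry into DestroyVolume has the game mode spawn a tile, then destroys this one; GetAttachLocation exposes the AttachPoint transform.
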(event `self.ReceiveBeginPlay`
  (`self.LockTile`)
  (`self.PlaceActors` "/Game/Dynamic/Terrain/SM_BP_Container.SM_BP_Container_C" 1 5 300.0 1.0 1.0)
  (`self.PlaceActors` "/Game/Dynamic/Terrain/S_Rock01_High_Blueprint.S_Rock01_High_Blueprint_C" 1 5 200.0 0.8 2.0)
  (`self.PlaceActors` "/Game/Dynamic/Terrain/S_Rock05_High_Blueprint.S_Rock05_High_Blueprint_C" 1 5 200.0 0.8 2.0)
  (`self.PlaceActors` "/Game/Dynamic/Terrain/S_Rock17_High_Blueprint.S_Rock17_High_Blueprint_C" 1 5 200.0 0.8 2.0)
  (`self.PlaceActors` "/Game/Dynamic/Terrain/SM_BP_Box.SM_BP_Box_C" 5 10 100.0 1.0 1.0 100.0)
  (`self.PlaceActors` "/Game/Dynamic/Terrain/SM_BP_Sandbag.SM_BP_Sandbag_C" 5 10 50.0 1.0 1.0 50.0)
  (`self.PlaceActors` "/Game/Dynamic/Terrain/SM_Canister_Blueprint.SM_Canister_Blueprint_C" 5 10 50.0 1.0 1.0 100.0)
  (`self.PlaceAICharacters` "/Game/Dynamic/Character/Behaviour/BP_Character.BP_Character_C" 2 4 100.0))

(event `self.LockingVolume.OnComponentBeginOverlap`
  (params (OverlappedComponent :type "PrimitiveComponent Object Reference") (OtherActor :type "Actor Object Reference") (OtherComp :type "PrimitiveComponent Object Reference") (OtherBodyIndex :type Integer) (bFromSweep :type Boolean) (SweepResult :type "HitResult Structure (by ref)"))
  (`self.isPlayerActor` OtherActor
    (:`true`
      (`self.UnlockTile`))))

(event `self.LockingVolume.OnComponentEndOverlap`
  (params (OverlappedComponent :type "PrimitiveComponent Object Reference") (OtherActor :type "Actor Object Reference") (OtherComp :type "PrimitiveComponent Object Reference") (OtherBodyIndex :type Integer))
  (`self.isPlayerActor` OtherActor
    (:`true`
      (`self.LockTile`))))

(event `self.DestroyVolume.OnComponentBeginOverlap`
  (params (OverlappedComponent :type "PrimitiveComponent Object Reference") (OtherActor :type "Actor Object Reference") (OtherComp :type "PrimitiveComponent Object Reference") (OtherBodyIndex :type Integer) (bFromSweep :type Boolean) (SweepResult :type "HitResult Structure (by ref)"))
  (`self.isPlayerActor` OtherActor
    (:`true`
      (bind _asinfinite_terrain_game_mode_bp (cast `/Game/Dynamic/InfiniteTerrainGameModeBP` (`GameplayStatics.GetGameMode`)))
      (`/Game/Dynamic/InfiniteTerrainGameModeBP.SpawnTile` _asinfinite_terrain_game_mode_bp)
      (`self.K2_DestroyActor`))))

(fn `GetAttachLocation`
  (returns (AttachTransform :type "Transform Structure"))
  (return (`SceneComponent.K2_GetComponentToWorld` (`self.AttachPoint`))))

(fn `LockTile`
  (`PrimitiveComponent.SetCollisionEnabled` (`self.BarrierStaticMesh`) "QueryAndPhysics")
  (`PrimitiveComponent.SetMaterial` (`self.BarrierStaticMesh`) 0 "/Game/Dynamic/Terrain/MI_Barrier_Red.MI_Barrier_Red"))

(fn `UnlockTile`
  (`PrimitiveComponent.SetCollisionEnabled` (`self.BarrierStaticMesh`) "NoCollision")
  (`PrimitiveComponent.SetMaterial` (`self.BarrierStaticMesh`) 0 "/Game/Dynamic/Terrain/MI_Barrier_Green.MI_Barrier_Green"))

(fn `UserConstructionScript`)