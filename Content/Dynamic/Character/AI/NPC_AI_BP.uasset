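; AI controller for guard NPCs that runs the GuardBehaviour tree on the PatrolData_New blackboard and reacts to perceiving the player.
; AI Perception updates are filtered by display name "Player1": non-hearing senses set EnemyKey to that actor, and failed senses clear it.
; Hearing only prints a debug message, as the stimulus-location write is disconnected.
; Targeting/shooting flags and a ChasePlayer tree switch are also left in unreachable nodes.
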(event `self.ReceiveBeginPlay`
  ;[1 1 1] Setup
  (bind _blackboardcomponent (`self.UseBlackboard` "/Game/Dynamic/Character/AI/PatrolData_New.PatrolData_New"))
  (`self.RunBehaviorTree` "/Game/Dynamic/Character/AI/GuardBehaviour.GuardBehaviour")
  (bind _output_get (set `self.Blacky` _blackboardcomponent))
  (`BlackboardComponent.ClearValue` _output_get (`self.EnemyKey`)))

(event `self.AIPerception.OnTargetPerceptionUpdated`
  (params (Actor :type "Actor Object Reference") (Stimulus :type "AIStimulus Structure"))
  (bind (_age _expirationage _strength _stimuluslocation _receiverlocation _tag _bsuccessfullysensed) (break `AIStimulus` Stimulus))
  (bind _returnvalue (`KismetSystemLibrary.GetDisplayName` Actor))
  (bind _returnvalue_2 (`KismetStringLibrary.Conv_VectorToString` _stimuluslocation))
  (bind _returnvalue_3 (`KismetSystemLibrary.GetDisplayName` (`self.K2_GetPawn`)))
  (if (`KismetStringLibrary.EqualEqual_StrStr` _returnvalue "Player1")
    (bind _returnvalue_4 (`AIPerceptionSystem.GetSenseClassForStimulus` Stimulus))
    (if (and (`KismetStringLibrary.NotEqual_StrStr` _returnvalue_3 _returnvalue) _bsuccessfullysensed)
      (if (`KismetStringLibrary.EqualEqual_StrStr` (`KismetSystemLibrary.GetClassDisplayName` _returnvalue_4) "AISense_Hearing")
        (bind _output_get (set `self.SenseType` " heard "))
        (`KismetSystemLibrary.PrintString` (`KismetStringLibrary.Concat_StrStr` _returnvalue_3 _output_get _returnvalue " at " _returnvalue_2) true true (struct :`R` 0.895 :`G` 0.271777 :`B` 0.02685 :`A` 1.0))
        (else
          (`BlackboardComponent.SetValueAsObject` (`self.Blacky`) (`self.EnemyKey`) Actor)
          (bind _output_get_2 (set `self.SenseType` " saw "))
          (`KismetSystemLibrary.PrintString` (`KismetStringLibrary.Concat_StrStr` _returnvalue_3 _output_get_2 _returnvalue " at " _returnvalue_2))))
      (else
        (`BlackboardComponent.ClearValue` (`self.Blacky`) (`self.EnemyKey`))))))

(event `self.ReceiveTick`
  (params (DeltaSeconds :type "Float (single-precision)")))

(fn `UserConstructionScript`)